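; AI controller for an enemy bot that runs BT_Bot and drives its Blackboard state: Passive, Investigating, Attack or Seeking.
; Perception updates turn seeing the player into Attack and losing sight into Seeking at the player's location.
; Any heard stimulus sets Investigating directly, even during Attack, bypassing the unused HandleSenseSound state check.
; A looping timer, started on possess, polls for forgotten seen actors, returning to Passive once the player is forgotten.
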(event `self.ReceiveBeginPlay`
  (`self.RunBehaviorTree` "/Game/AI/Enimies/Trees/BT_Bot.BT_Bot")
  (`self.SetStateAsPassive`))

(event `self.ReceivePossess`
  (params (PossessedPawn :type "Pawn Object Reference"))
  (bind _returnvalue (`KismetSystemLibrary.K2_SetTimerDelegate` (`|CreateDelegate` :!event `IfForgottenSeenActor`) 0.5 true))
  (set `self.CheckForgottenActorsTimer` _returnvalue))

(event `self.ReceiveUnPossess`
  (params (UnpossessedPawn :type "Pawn Object Reference"))
  (`KismetSystemLibrary.K2_ClearAndInvalidateTimerHandle` (`self.CheckForgottenActorsTimer`)))

(event `self.AIPerception.OnPerceptionUpdated`
  (params (UpdatedActors :type "Array of Actor Object Reference (by ref)"))
  (for _array_element UpdatedActors
    (`|ExecutionSequence`
      (:`then_0`
        (bind _issensed (`self.CanSenseActor` _array_element))
        (if _issensed
          (`self.HandleSenseSight` _array_element)
          (else
            (`self.HandleLostSight` _array_element))))
      (:`then_1`
        (bind (_issensed_2 _stimulus) (`self.CanSenseActor` _array_element "NewEnumerator1"))
        (if _issensed_2
          (`self.SetStateAsInvestigating` (`.StimulusLocation` (break `AIStimulus` _stimulus))))))))

(event `IfForgottenSeenActor`
  (if (!= (`KismetArrayLibrary.Array_Length` (`self.KnownSeenActors`)) (`KismetArrayLibrary.Array_Length` (`AIPerceptionComponent.GetKnownPerceivedActors` (`self.AIPerception`) "/Script/AIModule.AISense_Sight")))
    (for _array_element (`self.KnownSeenActors`)
      (if (== (`KismetArrayLibrary.Array_Find` (`AIPerceptionComponent.GetKnownPerceivedActors` (`self.AIPerception`) "/Script/AIModule.AISense_Sight") _array_element) -1)
        (`self.HandleForgotActor` _array_element)))))

(fn `CanSenseActor`
  (params (Actor :type "Actor Object Reference") (Sense :type "/Game/AI/Enimies/Enums/E_AI_Sense Enum" :default "NewEnumerator0"))
  (returns (isSensed :type Boolean) (Stimulus :type "AIStimulus Structure"))
  (bind _info (`AIPerceptionComponent.GetActorsPerception` (`self.AIPerception`) Actor))
  (for _array_element (`.LastSensedStimuli` (break `ActorPerceptionBlueprintInfo` _info))
    (bind _returnvalue (`AIPerceptionSystem.GetSenseClassForStimulus` _array_element))
    (if (== _returnvalue (select `/Game/AI/Enimies/Enums/E_AI_Sense` Sense :`NewEnumerator0` "/Script/AIModule.AISense_Sight" :`NewEnumerator1` "/Script/AIModule.AISense_Hearing" :`NewEnumerator2` "/Script/AIModule.AISense_Damage" :!type "AISense Class Reference"))
      (return (`.bSuccessfullySensed` (break `AIStimulus` _array_element)) _array_element))))

(fn `GetCurrentState`
  (returns (State :type "/Game/AI/Enimies/Enums/E_BotStates Enum"))
  (return (cast `/Game/AI/Enimies/Enums/E_BotStates` (`BlackboardComponent.GetValueAsEnum` (`AIBlueprintHelperLibrary.GetBlackboard` null) (`KismetStringLibrary.Conv_StringToName` "State")))))

(fn `HandleForgotActor`
  (params (Actor :type "Actor Object Reference"))
  (`KismetArrayLibrary.Array_RemoveItem` (`self.KnownSeenActors`) Actor)
  (if (== Actor (`GameplayStatics.GetPlayerCharacter` 0))
    (`self.SetStateAsPassive`)))

(fn `HandleLostSight`
  (params (Actor :type "Actor Object Reference"))
  (if (== Actor (`GameplayStatics.GetPlayerCharacter` 0))
    (bind _state (`self.GetCurrentState`))
    (switch `/Game/AI/Enimies/Enums/E_BotStates` _state
      (:`NewEnumerator1`
        _)
      (:`NewEnumerator3`
        _))
    (`self.SetStateAsSeeking` (`self.K2_GetActorLocation` (`GameplayStatics.GetPlayerCharacter` 0)))))

(fn `HandleSenseSight`
  (params (Actor :type "Actor Object Reference"))
  (if (== Actor (`GameplayStatics.GetPlayerCharacter` 0))
    (`KismetArrayLibrary.Array_AddUnique` (`self.KnownSeenActors`) Actor)
    (bind _state (`self.GetCurrentState`))
    (switch `/Game/AI/Enimies/Enums/E_BotStates` _state
      (:`NewEnumerator0`
        _)
      (:`NewEnumerator3`
        _)
      (:`NewEnumerator5`
        _))
    (`self.SetStateAsAttacking` Actor)))

(fn `HandleSenseSound`
  (params (Location :type "Vector Structure"))
  (bind _state (`self.GetCurrentState`))
  (switch `/Game/AI/Enimies/Enums/E_BotStates` _state
    (:`NewEnumerator0`
      _)
    (:`NewEnumerator3`
      _)
    (:`NewEnumerator5`
      _))
  (`self.SetStateAsInvestigating` Location))

(fn `SetStateAsAttacking`
  (params (AttackTarget :type "Actor Object Reference"))
  (bind _returnvalue (`AIBlueprintHelperLibrary.GetBlackboard` null))
  (`BlackboardComponent.SetValueAsEnum` _returnvalue (`KismetStringLibrary.Conv_StringToName` "State") (enumliteral `/Game/AI/Enimies/Enums/E_BotStates` "NewEnumerator1"))
  (`BlackboardComponent.SetValueAsObject` _returnvalue (`KismetStringLibrary.Conv_StringToName` "Player") AttackTarget))

(fn `SetStateAsInvestigating`
  (params (Location :type "Vector Structure"))
  (locals (State :type Name :default "State") (Point :type Name :default "PointOfInterest"))
  (bind _returnvalue (`AIBlueprintHelperLibrary.GetBlackboard` null))
  (`BlackboardComponent.SetValueAsEnum` _returnvalue (`KismetStringLibrary.Conv_StringToName` "State") (enumliteral `/Game/AI/Enimies/Enums/E_BotStates` "NewEnumerator3"))
  (`BlackboardComponent.SetValueAsVector` _returnvalue (`local.Point`) Location))

(fn `SetStateAsPassive`
  (`BlackboardComponent.SetValueAsEnum` (`AIBlueprintHelperLibrary.GetBlackboard` null) (`KismetStringLibrary.Conv_StringToName` "State") (enumliteral `/Game/AI/Enimies/Enums/E_BotStates` "NewEnumerator0")))

(fn `SetStateAsSeeking`
  (params (Location :type "Vector Structure"))
  (locals (State :type Name :default "State") (Point :type Name :default "PointOfInterest"))
  (bind _returnvalue (`AIBlueprintHelperLibrary.GetBlackboard` null))
  (`BlackboardComponent.SetValueAsEnum` _returnvalue (`local.State`) (enumliteral `/Game/AI/Enimies/Enums/E_BotStates` "NewEnumerator5"))
  (`BlackboardComponent.SetValueAsVector` _returnvalue (`local.Point`) Location))

(fn `UserConstructionScript`)