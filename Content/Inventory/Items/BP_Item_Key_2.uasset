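; BP_Item_Key_2 is an inventory item Blueprint for a key, with its data held in the ACItemData component.
; BeginPlay points that component at row "2" of the ItemData table, and LookAt reads the row to return a Russian "Take {Item}" prompt.
; Interaction is empty, Use only prints a placeholder message, and the LookAt call in the event graph is unconnected.
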(event `self.ReceiveBeginPlay`
  (set `/Game/Inventory/AC_Item_Data.ItemName` (make `DataTableRowHandle` "/Game/Inventory/ItemData.ItemData" "2") (`self.AC_Item_Data`)))

(event `self.InteractWith`
  (params (PlayerCharacter :type "/Game/FirstPerson/Blueprints/BP_FirstPersonCharacter Object Reference")))

(event `self.Use`
  (`KismetSystemLibrary.PrintString` "Implemented usage"))

(fn `LookAt`
  (returns (Message :type Text))
  (bind (_itemname_datatable _itemname_rowname) (break `DataTableRowHandle` (`/Game/Inventory/AC_Item_Data.ItemName` (`self.AC_Item_Data`))))
  (bind _returnvalue (`|GetDataTableRow` _itemname_datatable _itemname_rowname)
    (:`then`
      (return (`|FormatText` "Взять {Item}" (`KismetTextLibrary.Conv_NameToText` (`.Name_2_19A5DA2C4E8D35BC67435BBD5BE27503` (break `/Game/Inventory/FItemStruct` _returnvalue))))))
    (:`RowNotFound`
      (`KismetSystemLibrary.PrintText` "Not Found"))))

(fn `UserConstructionScript`)