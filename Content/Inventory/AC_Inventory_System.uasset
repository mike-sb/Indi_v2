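; Player inventory component that stores items as named slots and handles looking at, interacting with and using items.
; A sphere trace from the camera each tick tracks the looked-at actor and shows its message in a widget, and Interact triggers that actor's item data component.
; Slot names resolve through a data table, and consuming spawns the item's effect actor.
; Q sends a use message to the currently attached item.
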(event `self.ReceiveBeginPlay`
  (`KismetArrayLibrary.Array_Resize` (`self.Content`))
  (bind _returnvalue (`|CreateWidget` "/Game/Inventory/UI/UW_Message.UW_Message_C"))
  (bind _output_get (set `self.DisplayMessage` _returnvalue))
  (`UserWidget.AddToViewport` _output_get 0))

(event `self.ReceiveTick`
  (params (DeltaSeconds :type "Float (single-precision)"))
  (`self.InteractionTrace`))

(event `InputAction|Interact`
  (params (Key :type "Key Structure"))
  (:`Pressed`
    (bind _lookatactor (`self.LookAtActor`)
      (:`then`
        (bind _returnvalue (`Actor.GetComponentByClass` _lookatactor "/Game/Inventory/AC_Item_Data.AC_Item_Data_C"))
        (`/Engine/EditorBlueprintResources/StandardMacros.IsValid` _returnvalue
          (:`Is Valid`
            (bind _asbp_first_person_character (cast `/Game/FirstPerson/Blueprints/BP_FirstPersonCharacter` (`self.GetOwner`)))
            (message `/Game/Inventory/I_Interact.InteractWith` _returnvalue _asbp_first_person_character))))
      (:`else`))))

(event `ConsumeItemEvent`
  (params (Index :type Integer))
  (bind _output_itemname (break `/Game/Inventory/FSlotStruct` (`|GetArrayItem` (`self.Content`) Index)))
  (bind (_data_name _data_description _data_thumbnail _data_itemclass _data_itemeffect) (break `/Game/Inventory/FItemStruct` (`self.GetItemData` _output_itemname)))
  (bind _returnvalue (`|SpawnActorFromClass` _data_itemeffect (`Actor.GetTransform` (`GameplayStatics.GetPlayerController` 0)) "Undefined" "MultiplyWithRoot" null null))
  (`/Game/Inventory/Items/Effects/BP_Item_Effect.UseItem` _returnvalue _data_itemclass Index))

(event `Key|Q`
  (params (Key :type "Key Structure"))
  (:`Pressed`
    (if (`self.isAttached`)
      (bind _returnvalue (`GameplayStatics.GetActorOfClass` (`self.attachedItem`)))
      (message `/Game/Inventory/I_Interact.Use` _returnvalue))))

(fn `AddToInventory`
  (params (ItemName :type Name))
  (`KismetArrayLibrary.Array_Add` (`self.Content`) (make `/Game/Inventory/FSlotStruct` ItemName)))

(fn `FindItemIndex`
  (params (ItemName :type Name))
  (returns (Index :type Integer))
  (for (_array_element _array_index) (`self.Content`)
    (if (== ItemName (break `/Game/Inventory/FSlotStruct` _array_element))
      (return _array_index)))
  (return -1))

(fn `GetAttachedState`
  (returns (isAttached :type Boolean) (item :type "Actor Class Reference"))
  (return (`self.isAttached`) (`self.attachedItem`)))

(fn `GetItemData`
  (params (ItemName :type Name))
  (returns (Data :type "/Game/Inventory/FItemStruct Structure"))
  (bind _returnvalue (`|GetDataTableRow` "/Game/Inventory/ItemData.ItemData" ItemName)
    (:`then`
      (return _returnvalue))))

(fn `InteractionTrace`
  (bind _returnvalue (`GameplayStatics.GetPlayerCameraManager` 0))
  (bind _returnvalue_2 (`Actor.K2_GetActorLocation` _returnvalue))
  (bind (_outhit _returnvalue_3) (`KismetSystemLibrary.SphereTraceSingle` _returnvalue_2 (+ _returnvalue_2 (* (`Actor.GetActorForwardVector` _returnvalue) 300.0)) 10.0 "TraceTypeQuery3" false (`|MakeArray` (`self.GetOwner`)) "ForOneFrame"))
  (if _returnvalue_3
    (bind (_bblockinghit _binitialoverlap _time _distance _location _impactpoint _normal _impactnormal _physmat _hitactor) (`GameplayStatics.BreakHitResult` _outhit))
    (if (!= _hitactor (`self.LookAtActor`))
      (bind _output_get (set `self.LookAtActor` _hitactor))
      (bind _message (message `/Game/Inventory/I_Interact.LookAt` _output_get))
      (`/Game/Inventory/UI/UW_Message.ShowMessage` (`self.DisplayMessage`) _message))
    (else
      (set `self.LookAtActor` _hitactor)
      (`/Game/Inventory/UI/UW_Message.ShowMessage` (`self.DisplayMessage`) ""))))

(fn `QueryInventory`
  (params (ItemName :type Name))
  (returns (Success :type Boolean))
  (for _array_element (`self.Content`)
    (if (== (`.ItemName_2_2FB955374C48E52C444F6986B679A6E8` (break `/Game/Inventory/FSlotStruct` _array_element)) ItemName)
      (return true)))
  (return false))

(fn `RemoveItem`
  (params (Index :type Integer))
  (locals (`Local Item Name` :type Name))
  (bind _content (`self.Content`))
  (bind _output_itemname (break `/Game/Inventory/FSlotStruct` (`|GetArrayItem` _content Index)))
  (set `local.Local Item Name` _output_itemname)
  (`KismetArrayLibrary.Array_Remove` _content Index))

(fn `SetAttachedState`
  (params (item :type "Actor Class Reference") (isAttached :type Boolean))
  (set `self.attachedItem` item)
  (set `self.isAttached` isAttached))